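; Player character for a side-scrolling game, moved along X with a jump, and pinned to Y = 0 every Tick.
; Hitting an EnemyBlueprint sets HitByEnemy, and overlapping a LevelPickupBlueprint calls the FirstPickupDispatch dispatcher.
; ApplyFallDamage cuts health on high downward velocity and reloads the level at zero or below, but is unwired: OnLanded is empty.
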(event `self.ReceiveTick`
  (params (DeltaSeconds :type "Float (single-precision)"))
  (bind (_returnvalue_x _returnvalue_y _returnvalue_z) (`KismetMathLibrary.BreakVector` (`self.K2_GetActorLocation`)))
  ;[1 1 1] Fix actor location
  (`self.K2_SetActorLocation` (`KismetMathLibrary.MakeVector` _returnvalue_x 0.0 _returnvalue_z)))

(event `InputAction|DoJump`
  (params (Key :type "Key Structure" :default "AnyKey"))
  ;[1 1 1] Basic Movement
  (:`Pressed`
    (`self.Jump`))
  (:`Released`
    (`self.StopJumping`)))

(event `InputAxis|DoMoveLeft`
  (params (AxisValue :type "Float (single-precision)"))
  ;[1 1 1] Basic Movement
  (`self.AddMovementInput` (1.0 0.0 0.0) AxisValue))

(event `self.ReceiveHit`
  (params (MyComp :type "PrimitiveComponent Object Reference") (Other :type "Actor Object Reference") (OtherComp :type "PrimitiveComponent Object Reference") (bSelfMoved :type Boolean) (HitLocation :type "Vector Structure") (HitNormal :type "Vector Structure") (NormalImpulse :type "Vector Structure") (Hit :type "HitResult Structure (by ref)"))
  ;[1 1 1] Enemy possession
  (if (== (`GameplayStatics.GetObjectClass` Other) "/Game/Blueprints/CharacterBlueprints/EnemyBlueprint.EnemyBlueprint_C")
    (set `self.bHitByEnemy` true)))

(event `self.OnLanded`
  (params (Hit :type "HitResult Structure (by ref)"))
  ;[1 1 1] Fall Damage
)

(event `self.ReceiveActorBeginOverlap`
  (params (OtherActor :type "Actor Object Reference"))
  (if (== (`GameplayStatics.GetObjectClass` OtherActor) "/Game/Blueprints/ObjectBlueprints/LevelPickupBlueprint.LevelPickupBlueprint_C")
    (`self.FirstPickupDispatch`)))

(fn `ApplyFallDamage`
  (bind (_velocity_x _velocity_y _velocity_z) (`KismetMathLibrary.BreakVector` (`MovementComponent.Velocity` (`self.CharacterMovement`))))
  (bind _returnvalue (* _velocity_z -1.0))
  (`/Engine/EditorBlueprintResources/StandardMacros.CompareFloat` _returnvalue 10000.0
    (:`>`
      (set `self.PlayerHealth` (- (`self.PlayerHealth`) (* _returnvalue 0.001)))
      (`KismetSystemLibrary.PrintString` (`KismetStringLibrary.Conv_DoubleToString` (`self.PlayerHealth`)))
      (`/Engine/EditorBlueprintResources/StandardMacros.CompareFloat` (`self.PlayerHealth`)
        (:`==`
          _)
        (:`<`
          _))
      (`self.K2_DestroyActor`)
      (bind _returnvalue_2 (`GameplayStatics.GetCurrentLevelName` true))
      (`GameplayStatics.OpenLevel` (`KismetStringLibrary.Conv_StringToName` _returnvalue_2)))))

(fn `UserConstructionScript`)