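; Second playable character Blueprint for a side-scrolling game, locked to the Y=0 plane every tick, with axis movement and a boosted jump.
; Its special throws a magnet toward the deprojected mouse position, lerping it there on a timeline before enabling its tick.
; Only one magnet exists at a time, and it is destroyed after a delay.
; Overlapping a level pickup fires the second-pickup dispatcher.
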(event `self.ReceiveTick`
  (params (DeltaSeconds :type "Float (single-precision)"))
  (bind (_returnvalue_x _returnvalue_y _returnvalue_z) (`KismetMathLibrary.BreakVector` (`self.K2_GetActorLocation`)))
  ;[1 1 1] Fix Actor Location
  (`self.K2_SetActorLocation` (`KismetMathLibrary.MakeVector` _returnvalue_x 0.0 _returnvalue_z)))

(event `InputAction|DoJump`
  (params (Key :type "Key Structure" :default "AnyKey"))
  ;[1 1 1] Basic Movement
  (:`Pressed`
    (`self.Jump`))
  (:`Released`
    (`self.StopJumping`)))

(event `InputAxis|DoMoveLeft`
  (params (AxisValue :type "Float (single-precision)"))
  ;[1 1 1] Basic Movement
  (`self.AddMovementInput` (1.0 0.0 0.0) AxisValue))

(event `InputAction|Special`
  (params (Key :type "Key Structure" :default "AnyKey"))
  (bind _worldlocation (`PlayerController.DeprojectMousePositionToWorld` (`GameplayStatics.GetPlayerController` 0)))
  ;[1 1 1] Magnet
  (:`Pressed`
    (set `self.MagnetLocation` (`KismetMathLibrary.MakeVector` (.x _worldlocation) 0.0 (.z _worldlocation)))
    (if (not (`self.bHasThrownMagnet`))
      (bind _returnvalue (`|SpawnActorFromClass` "/Game/Blueprints/ObjectBlueprints/MagnetBP.MagnetBP_C" (`KismetMathLibrary.MakeTransform` (`self.K2_GetActorLocation`)) "Undefined" "OverrideRootScale" self self))
      (`self.SetActorTickEnabled` _returnvalue false)
      (set `self.bHasThrownMagnet` true)
      (set `self.Special` "Checked")
      (bind (_direction _floattimeline) (`Timeline|ThrowMagnetTimeline` :!via `PlayFromStart`)
        (:`Update`
          (`self.K2_SetActorLocation` _returnvalue (`KismetMathLibrary.VLerp` (`self.K2_GetActorLocation`) (`self.MagnetLocation`) _floattimeline) false false))
        (:`Finished`
          (bind _output_get (set `self.MagnetReference` _returnvalue))
          (`self.SetActorTickEnabled` _output_get true)
          (`KismetSystemLibrary.Delay` 20.0)
          (set `self.bHasThrownMagnet` false)
          (set `self.Special` "Unchecked")
          (`self.K2_DestroyActor` _returnvalue))))))

(event `self.ReceiveActorBeginOverlap`
  (params (OtherActor :type "Actor Object Reference"))
  (if (== (`GameplayStatics.GetObjectClass` OtherActor) "/Game/Blueprints/ObjectBlueprints/LevelPickupBlueprint.LevelPickupBlueprint_C")
    (`self.SecondPickupDispatch`)))

(event `self.ReceiveBeginPlay`
  ;[1 1 1] Setting jump height/velocity. Default 420
  (set `CharacterMovementComponent.JumpZVelocity` 600.0 (`self.CharacterMovement`)))

(fn `UserConstructionScript`)