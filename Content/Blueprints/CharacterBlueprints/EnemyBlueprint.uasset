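; Side-scrolling enemy character that patrols along X and can also take player jump and move input.
; Tick pins Y to zero and, while IdleMove is set, walks in a direction that flips on each Hit.
; Overlap zeroes PlayerHealth on the Second and Third character Blueprints, sparing the First.
; UnpossessedByPlayer re-enables IdleMove after a delay; nothing here clears it, and the rotation nodes are unwired.
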(event `self.ReceiveBeginPlay`
  (set `self.bIdleMove` true))

(event `InputAxis|DoMoveLeft`
  (params (AxisValue :type "Float (single-precision)"))
  ;[1 1 1] PlayerControl Movement
  (`self.AddMovementInput` (1.0 0.0 0.0) AxisValue))

(event `InputAction|DoJump`
  (params (Key :type "Key Structure" :default "AnyKey"))
  ;[1 1 1] PlayerControl Movement
  (:`Pressed`
    (`self.Jump`))
  (:`Released`
    (`self.StopJumping`)))

(event `self.ReceiveActorBeginOverlap`
  (params (OtherActor :type "Actor Object Reference"))
  (bind _returnvalue (`GameplayStatics.GetObjectClass` OtherActor))
  ;[1 1 1] Player health damage on overlap
  (if (== _returnvalue "/Game/Blueprints/CharacterBlueprints/FirstCharacterBlueprint.FirstCharacterBlueprint_C")
    _
    (elif (== _returnvalue "/Game/Blueprints/CharacterBlueprints/SecondCharacterBlueprint.SecondCharacterBlueprint_C")
      (bind _assecond_character_blueprint (cast `/Game/Blueprints/CharacterBlueprints/SecondCharacterBlueprint` OtherActor))
      (set `/Game/Blueprints/CharacterBlueprints/SecondCharacterBlueprint.PlayerHealth` 0.0 _assecond_character_blueprint)
      (elif (== _returnvalue "/Game/Blueprints/CharacterBlueprints/ThirdCharacterBlueprint.ThirdCharacterBlueprint_C")
        (bind _asthird_character_blueprint (cast `/Game/Blueprints/CharacterBlueprints/ThirdCharacterBlueprint` OtherActor))
        (set `/Game/Blueprints/CharacterBlueprints/ThirdCharacterBlueprint.PlayerHealth` 0.0 _asthird_character_blueprint)))))

(event `Unpossessed By Player`
  ;[1 1 1] Restart idle movement X seconds after being unpossessed
  (`KismetSystemLibrary.PrintString` "Waiting 5 seconds")
  (`KismetSystemLibrary.Delay` 5.0)
  (set `self.bIdleMove` true)
  (`KismetSystemLibrary.PrintString` "Idle Move on"))

(event `self.ReceiveHit`
  (params (MyComp :type "PrimitiveComponent Object Reference") (Other :type "Actor Object Reference") (OtherComp :type "PrimitiveComponent Object Reference") (bSelfMoved :type Boolean) (HitLocation :type "Vector Structure") (HitNormal :type "Vector Structure") (NormalImpulse :type "Vector Structure") (Hit :type "HitResult Structure (by ref)"))
  (bind _benemymovedirection (`self.bEnemyMoveDirection`))
  ;[1 1 1] Enemy Hit Detection and Direction Change
  (if _benemymovedirection
    _
    (else
      _))
  (set `self.bEnemyMoveDirection` (not _benemymovedirection)))

(event `self.ReceiveTick`
  (params (DeltaSeconds :type "Float (single-precision)"))
  (bind (_returnvalue_x _returnvalue_y _returnvalue_z) (`KismetMathLibrary.BreakVector` (`self.K2_GetActorLocation`)))
  ;[1 1 1] Idle movement
  (`self.K2_SetActorLocation` (`KismetMathLibrary.MakeVector` _returnvalue_x 0.0 _returnvalue_z))
  (if (`self.bIdleMove`)
    ;;[1 1 1] Check current direction. 0=left,1=right
    (if (`self.bEnemyMoveDirection`)
      (`self.AddMovementInput` (`KismetMathLibrary.MakeVector` 1.0) 0.2)
      (else
        (`self.AddMovementInput` (`KismetMathLibrary.MakeVector` -1.0) 0.2)))))

(fn `UserConstructionScript`)