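; Side-scrolling player character that moves along X, jumps, and grows a climbable vine up to ledges overhead.
; Special traces upward for a LedgeBlueprint and spawns a VineBlueprint scaled to the gap, replacing any existing one and expiring after a delay.
; Overlapping a vine snaps X to it without sideways input; climbing requires Flying mode, which is set outside this graph.
; Tick pins Y to zero; vine expiry restores Walking and ledge collision.
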(event `self.ReceiveActorBeginOverlap`
  (params (OtherActor :type "Actor Object Reference"))
  (bind (_returnvalue_x _returnvalue_y _returnvalue_z) (`KismetMathLibrary.BreakVector` (`self.K2_GetActorLocation`)))
  (bind _returnvalue_x_2 (`KismetMathLibrary.BreakVector` (`self.K2_GetActorLocation` OtherActor)))
  ;[1 1 1] Lock actor to vine when overlapping it
  (if (== (`GameplayStatics.GetObjectClass` OtherActor) "/Game/Blueprints/ObjectBlueprints/VineBlueprint.VineBlueprint_C")
    (`self.K2_SetActorLocation` (`KismetMathLibrary.MakeVector` _returnvalue_x_2 0.0 _returnvalue_z))
    (set `self.bIsOverlappingVine` true)
    (set `self.VineReference` OtherActor)))

(event `self.ReceiveActorEndOverlap`
  (params (OtherActor :type "Actor Object Reference"))
  ;[1 1 1] Free actor from vine when not overlapping
  (if (== (`GameplayStatics.GetObjectClass` OtherActor) "/Game/Blueprints/ObjectBlueprints/VineBlueprint.VineBlueprint_C")
    (set `self.bIsOverlappingVine` false)))

(event `InputAction|Special`
  (params (Key :type "Key Structure" :default "AnyKey"))
  (bind (_returnvalue_x _returnvalue_y _returnvalue_z) (`KismetMathLibrary.BreakVector` (`self.K2_GetActorLocation`)))
  (bind (_returnvalue_x_2 _returnvalue_y_2 _returnvalue_z_2) (`KismetMathLibrary.BreakVector` (`self.K2_GetActorLocation`)))
  ;[1 1 1] Spawn Vine
  (:`Pressed`
    (if (`self.bIsVineExisting`)
      (`self.K2_DestroyActor` (`self.VineReference`))
      (`self.SetActorEnableCollision` (`self.LedgeReference`) true)
      (set `self.bIsVineExisting` false)
      (set `self.VineReference` null)
      (set `self.LedgeReference` null))
    (bind _outactors (`GameplayStatics.GetAllActorsOfClass` "/Game/Blueprints/ObjectBlueprints/LedgeCollisionOffBlueprint.LedgeCollisionOffBlueprint_C"))
    (bind _outhit (`KismetSystemLibrary.LineTraceSingleForObjects` (`self.K2_GetActorLocation`) (+ (`self.K2_GetActorLocation`) (0.0 0.0 1024.0)) (`self.ObjectTypes`) false _outactors))
    (if (== (`GameplayStatics.GetObjectClass` (`.HitActor` (`GameplayStatics.BreakHitResult` _outhit))) "/Game/Blueprints/ObjectBlueprints/LedgeBlueprint.LedgeBlueprint_C")
      (set `self.LedgeReference` (`.HitActor` (`GameplayStatics.BreakHitResult` _outhit)))
      (bind _returnvalue (+ (/ (- (* _returnvalue_z -1.0) (* (.z (`.Location` (`GameplayStatics.BreakHitResult` _outhit))) -1.0)) 32.0) 1.0))
      (bind _returnvalue_2 (`|SpawnActorFromClass` "/Game/Blueprints/ObjectBlueprints/VineBlueprint.VineBlueprint_C" (`KismetMathLibrary.MakeTransform` (`KismetMathLibrary.MakeVector` _returnvalue_x_2 0.0 (+ _returnvalue_z_2 (* _returnvalue 16.0))) (struct) (`KismetMathLibrary.MakeVector` 1.0 1.0 _returnvalue)) "Undefined" "OverrideRootScale"))
      (set `self.bIsVineExisting` true)
      (`KismetSystemLibrary.Delay` 10.0)
      (`self.K2_DestroyActor` _returnvalue_2)
      (`CharacterMovementComponent.SetMovementMode` (`self.CharacterMovement`) "MOVE_Walking" 0)
      (`KismetSystemLibrary.Delay` 0.5)
      (`self.SetActorEnableCollision` (`self.LedgeReference`) true)
      (set `self.VineReference` null)
      (set `self.LedgeReference` null)
      (set `self.bIsVineExisting` false))))

(event `InputAxis|DoMoveLeft`
  (params (AxisValue :type "Float (single-precision)"))
  ;[1 1 1] Basic Movement
  (`self.AddMovementInput` (1.0 0.0 0.0) AxisValue))

(event `InputAxis|ClimbUp`
  (params (AxisValue :type "Float (single-precision)"))
  ;[1 1 1] Climb up vine
  (`/Engine/EditorBlueprintResources/StandardMacros.CompareFloat` AxisValue
    (:`>`
      (if (`|EnumEquality` (`CharacterMovementComponent.MovementMode` (`self.CharacterMovement`)) "MOVE_Flying")
        (`self.AddMovementInput` (0.0 0.0 0.2))))
    (:`==`
      (if (`self.IsOverlappingActor` (`self.VineReference`))
        (`/Engine/EditorBlueprintResources/StandardMacros.CompareFloat` (`self.GetInputAxisValue`)
          (:`==`
            (set `MovementComponent.Velocity` (0.0 0.0 0.0) (`self.CharacterMovement`))))))))

(event `self.ReceiveTick`
  (params (DeltaSeconds :type "Float (single-precision)"))
  (bind (_returnvalue_x _returnvalue_y _returnvalue_z) (`KismetMathLibrary.BreakVector` (`self.K2_GetActorLocation`)))
  (bind (_returnvalue_x_2 _returnvalue_y_2 _returnvalue_z_2) (`KismetMathLibrary.BreakVector` (`self.K2_GetActorLocation`)))
  (bind _returnvalue_x_3 (`KismetMathLibrary.BreakVector` (`self.K2_GetActorLocation` (`self.VineReference`))))
  ;[1 1 1] Fix actor location as long as vine overlapping
  (`self.K2_SetActorLocation` (`KismetMathLibrary.MakeVector` _returnvalue_x 0.0 _returnvalue_z))
  (if (`self.bIsOverlappingVine`)
    (`/Engine/EditorBlueprintResources/StandardMacros.CompareFloat` (`self.GetInputAxisValue`)
      (:`==`
        (`self.K2_SetActorLocation` (`KismetMathLibrary.MakeVector` _returnvalue_x_3 0.0 _returnvalue_z_2))))))

(event `InputAction|DoJump`
  (params (Key :type "Key Structure" :default "AnyKey"))
  ;[1 1 1] Basic Movement
  (:`Pressed`
    (`self.Jump`))
  (:`Released`
    (`self.StopJumping`)))

(fn `UserConstructionScript`)