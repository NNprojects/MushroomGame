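; VineBlueprint is a climbable vine trigger that lets the third-person player character move freely while overlapping it.
; On begin overlap with a ThirdCharacterBlueprint, it switches that character's movement mode to Flying.
; On end overlap, it sets the mode back to Walking; climb input and direction are not handled here.
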(event `self.ReceiveActorBeginOverlap`
  (params (OtherActor :type "Actor Object Reference"))
  (if (== (`GameplayStatics.GetObjectClass` OtherActor) "/Game/Blueprints/CharacterBlueprints/ThirdCharacterBlueprint.ThirdCharacterBlueprint_C")
    (bind _asthird_character_blueprint (cast `/Game/Blueprints/CharacterBlueprints/ThirdCharacterBlueprint` OtherActor))
    (`CharacterMovementComponent.SetMovementMode` (`Character.CharacterMovement` _asthird_character_blueprint) "MOVE_Flying" 0)))

(event `self.ReceiveActorEndOverlap`
  (params (OtherActor :type "Actor Object Reference"))
  (if (== (`GameplayStatics.GetObjectClass` OtherActor) "/Game/Blueprints/CharacterBlueprints/ThirdCharacterBlueprint.ThirdCharacterBlueprint_C")
    (bind _asthird_character_blueprint (cast `/Game/Blueprints/CharacterBlueprints/ThirdCharacterBlueprint` OtherActor))
    (`CharacterMovementComponent.SetMovementMode` (`Character.CharacterMovement` _asthird_character_blueprint) "MOVE_Walking" 0)))

(fn `UserConstructionScript`)