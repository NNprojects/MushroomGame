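; Magnet actor that captures overlapping EnemyBlueprint actors and pulls them toward itself.
; Begin overlap adds each enemy to an array and switches it to Flying movement, and destroying the magnet sets them all back to Walking.
; Tick restarts one shared timeline for each stored enemy, whose update calls Magnet to lerp location toward the magnet, feeding only X and Z.
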(event `self.ReceiveDestroyed`
  (for _array_element (`self.ArrayOfMagneticObjectReferences`)
    (`CharacterMovementComponent.SetMovementMode` (`Character.CharacterMovement` _array_element) "MOVE_Walking" 0)))

(event `self.ReceiveTick`
  (params (DeltaSeconds :type "Float (single-precision)"))
  (for _array_element (`self.ArrayOfMagneticObjectReferences`)
    (bind (_direction _alphafloat) (`Timeline|Timeline_0` :!via `PlayFromStart`)
      (:`Update`
        (`self.Magnet` _alphafloat _array_element)))))

(event `self.ReceiveActorBeginOverlap`
  (params (OtherActor :type "Actor Object Reference"))
  (if (== (`GameplayStatics.GetObjectClass` OtherActor) "/Game/Blueprints/CharacterBlueprints/EnemyBlueprint.EnemyBlueprint_C")
    (bind _asenemy_blueprint (cast `/Game/Blueprints/CharacterBlueprints/EnemyBlueprint` OtherActor))
    (`KismetArrayLibrary.Array_AddUnique` (`self.ArrayOfMagneticObjectReferences`) _asenemy_blueprint)
    (`CharacterMovementComponent.SetMovementMode` (`Character.CharacterMovement` _asenemy_blueprint) "MOVE_Flying" 0)))

(fn `Magnet`
  (params (Alpha :type "Float (double-precision)") (ActorReference :type "Actor Object Reference"))
  (bind (_returnvalue_x _returnvalue_y _returnvalue_z) (`KismetMathLibrary.BreakVector` (`KismetMathLibrary.VLerp` (`self.K2_GetActorLocation` ActorReference) (`self.K2_GetActorLocation` self) Alpha)))
  ;[1 1 1] Pull actor towards magnet
  (if (== (`GameplayStatics.GetObjectClass` ActorReference) "/Game/Blueprints/CharacterBlueprints/EnemyBlueprint.EnemyBlueprint_C")
    (if (`KismetSystemLibrary.IsValid` ActorReference)
      (`self.K2_SetActorLocation` ActorReference (`KismetMathLibrary.MakeVector` _returnvalue_x 0.0 _returnvalue_z) false false))))

(fn `UserConstructionScript`)