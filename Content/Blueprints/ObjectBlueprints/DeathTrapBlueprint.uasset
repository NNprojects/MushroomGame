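; DeathTrapBlueprint is a trap actor that instantly kills any of the three player characters that overlaps it.
; On ActorBeginOverlap it compares the other actor's class against the First, Second and Third character Blueprints in a nested branch chain.
; The matching branch casts the actor, sets its PlayerHealth to zero and prints an on-screen debug message.
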(event `self.ReceiveActorBeginOverlap`
  (params (OtherActor :type "Actor Object Reference"))
  (bind _returnvalue (`GameplayStatics.GetObjectClass` OtherActor))
  (if (== _returnvalue "/Game/Blueprints/CharacterBlueprints/FirstCharacterBlueprint.FirstCharacterBlueprint_C")
    (bind _asfirst_character_blueprint (cast `/Game/Blueprints/CharacterBlueprints/FirstCharacterBlueprint` OtherActor))
    (set `/Game/Blueprints/CharacterBlueprints/FirstCharacterBlueprint.PlayerHealth` 0.0 _asfirst_character_blueprint)
    (`KismetSystemLibrary.PrintString` "Health 0!" true true (struct :`G` 0.66 :`B` 1.0 :`A` 1.0) 5.0 :!label _label)
    (elif (== _returnvalue "/Game/Blueprints/CharacterBlueprints/SecondCharacterBlueprint.SecondCharacterBlueprint_C")
      (bind _assecond_character_blueprint (cast `/Game/Blueprints/CharacterBlueprints/SecondCharacterBlueprint` OtherActor))
      (set `/Game/Blueprints/CharacterBlueprints/SecondCharacterBlueprint.PlayerHealth` 0.0 _assecond_character_blueprint)
      (goto _label)
      (elif (== _returnvalue "/Game/Blueprints/CharacterBlueprints/ThirdCharacterBlueprint.ThirdCharacterBlueprint_C")
        (bind _asthird_character_blueprint (cast `/Game/Blueprints/CharacterBlueprints/ThirdCharacterBlueprint` OtherActor))
        (set `/Game/Blueprints/CharacterBlueprints/ThirdCharacterBlueprint.PlayerHealth` 0.0 _asthird_character_blueprint)
        (goto _label)))))

(fn `UserConstructionScript`)